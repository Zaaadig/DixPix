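; BP_TargetPointZone is a target point trigger that steers BP_Pickable movement through a Sphere overlap.
; Overlap begin sets the pickable's OutOfTargetPoint flag to true, and overlap end clears it.
; For one fruit type, it also removes itself from the pickable's TempAllTargetPoints, then calls MovementFromTargetPoint after a short delay.
; The delayed call uses the shared CurrentPickable variable, which any later overlap overwrites.
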(event OnComponentBeginOverlap(Sphere)
  (params (OverlappedComponent :type Primitive%20Component%20Object%20Reference) (OtherActor :type Actor%20Object%20Reference) (OtherComp :type Primitive%20Component%20Object%20Reference) (OtherBodyIndex :type Integer) (bFromSweep :type Boolean) (SweepResult :type Hit%20Result%20Structure%20%28by%20ref%29))
  (bind _asbp_pickable (Utilities|Casting|CastToBP_Pickable OtherActor))
  (bind _output_get (Variables|Default|SetCurrentPickable _asbp_pickable))
  (Variables|/Game/Blueprints/Pickable/BP_Pickable.BP_Pickable_C|SetbOutOfTargetPoint _output_get true)
  (if (and (Utilities|Enum|Equal(Enum) (Variables|/Game/Blueprints/Pickable/BP_Pickable.BP_Pickable_C|GetFruitsTypeChosen _asbp_pickable) "NewEnumerator2") (Variables|/Game/Blueprints/Pickable/BP_Pickable.BP_Pickable_C|GetbOutOfTargetPoint (Variables|Default|GetCurrentPickable)))
    (Utilities|Array|RemoveItem (Variables|/Game/Blueprints/Pickable/BP_Pickable.BP_Pickable_C|GetTempAllTargetPoints (Variables|Default|GetCurrentPickable)) self)
    (Utilities|FlowControl|Delay 0.2)
    (Default|MovementfromTargetPoint (Variables|Default|GetCurrentPickable))))

(event OnComponentEndOverlap(Sphere)
  (params (OverlappedComponent :type Primitive%20Component%20Object%20Reference) (OtherActor :type Actor%20Object%20Reference) (OtherComp :type Primitive%20Component%20Object%20Reference) (OtherBodyIndex :type Integer))
  (bind _asbp_pickable (Utilities|Casting|CastToBP_Pickable OtherActor))
  (Variables|/Game/Blueprints/Pickable/BP_Pickable.BP_Pickable_C|SetbOutOfTargetPoint _asbp_pickable false))

(event EventBeginPlay)

(event Collision|EventActorBeginOverlap
  (params (OtherActor :type Actor%20Object%20Reference)))

(event EventTick
  (params (DeltaSeconds :type Float%20%28single-precision%29)))

(fn ConstructionScript)