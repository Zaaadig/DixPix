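; BP_GameManager is a game manager that puts up the countdown timer and holds the player's objective.
; On BeginPlay it creates a WB_Timer widget, sets its starting time left to two minutes (120) and adds it to the viewport.
; The RecupPlayerObjectif event stores the Menager, Fruits and Frais inputs and packs them into an SObjectif struct saved as Objectif.
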(event Custom|RecupPlayerObjectif
  (params (Menager :type E_MenagerType%20Enum :default "NewEnumerator0") (Fruits :type E_FruitsType%20Enum :default "NewEnumerator0") (Frais :type E_FraisType%20Enum :default "NewEnumerator0"))
  (Variables|Default|SetMenager Menager)
  (Variables|Default|SetFruits Fruits)
  (Variables|Default|SetFrais Frais)
  (Variables|Default|SetObjectif (Utilities|Struct|MakeS_Objectif (Variables|Default|GetMenager) (Variables|Default|GetFruits) (Variables|Default|GetFrais))))

(event EventBeginPlay
  (bind _returnvalue (UserInterface|CreateWidget "/Game/UI/WB_Timer.WB_Timer_C"))
  (bind _output_get (Variables|Timer|SetWB_Timer _returnvalue))
  (Variables|/Game/UI/WB_Timer.WB_Timer_C|SetTimeLeft _output_get 120)
  (UserInterface|Viewport|AddtoViewport (Variables|Timer|GetWB_Timer) 0))

(fn ConstructionScript)