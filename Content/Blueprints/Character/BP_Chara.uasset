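; Auto-running player caddie character that moves forward every tick, with Enhanced Input for strafing, jumping and slowing.
; Holding slow lowers Speed and triggers a resource check that drains Ressource, forces StopSlow when empty and starts timer-based regen.
; Box overlaps with BP_Pickable play a timeline pulling the item along a spline while shrinking it and wobbling the caddie, then activate Niagara and destroy it.
; A self-restarting timeline pulses the Cube's scale as idle animation.
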(event OnComponentBeginOverlap(Box)
  (params (OverlappedComponent :type Primitive%20Component%20Object%20Reference) (OtherActor :type Actor%20Object%20Reference) (OtherComp :type Primitive%20Component%20Object%20Reference) (OtherBodyIndex :type Integer) (bFromSweep :type Boolean) (SweepResult :type Hit%20Result%20Structure%20%28by%20ref%29))
  (bind _asbp_pickable (Utilities|Casting|CastToBP_Pickable OtherActor))
  (bind _output_get (Variables|Default|SetCurrentPickup _asbp_pickable))
  (Utilities|Array|Add (Variables|Defaults|GetListAllItemsPickup) _output_get)
  (Variables|Default|SetStartRotationCaddiePickup (Transformation|GetActorRotation))
  (Variables|Default|SetStartCameraRotationPickup (Transformation|GetActorRotation (Variables|Default|GetMainCamera)))
  (Variables|Default|SetWorldScaleCaddie (Transformation|GetWorldScale (Variables|Default|GetCube)))
  (Utilities|IsValid (Variables|Default|GetCurrentPickup)
    (:Is%20Valid
      (Collision|SetActorEnableCollision (Variables|Default|GetCurrentPickup) false)
      (Components|Timeline|SetPlayRate (Variables|Default|GetTL_Pickup) (/ 1.0 0.75))
      (bind (_direction _alpha _rotation) (Timeline|TL_Pickup PlayFromStart)
        (:Update
          (Transformation|SetActorLocation (Variables|Default|GetCurrentPickup) (Spline|GetLocationatTime (Variables|Default|GetSplinePickup) _alpha "World" false) false false)
          (Transformation|SetActorScale3D (Variables|Default|GetCurrentPickup) (Math|Vector|Lerp(Vector) "1.000000,1.000000,1.000000" "0, 0, 0" _alpha))
          (Transformation|SetActorRotation (Math|Rotator|MakeRotator (.roll (Math|Rotator|Lerp(Rotator) (Math|Rotator|CombineRotators (Variables|Default|GetStartRotationCaddiePickup) "10.000000,0.000000,0.000000") (Math|Rotator|CombineRotators (Variables|Default|GetStartRotationCaddiePickup) "-10.000000,0.000000,0.000000") _rotation true)) (.pitch (Variables|Default|GetStartRotationCaddiePickup)) (.yaw (Math|Rotator|Lerp(Rotator) (Math|Rotator|CombineRotators (Variables|Default|GetStartRotationCaddiePickup) "10.000000,0.000000,0.000000") (Math|Rotator|CombineRotators (Variables|Default|GetStartRotationCaddiePickup) "-10.000000,0.000000,0.000000") _rotation true)))))
        (:Finished
          (Components|Activation|Activate (Variables|Default|GetNiagara) true)
          (Actor|DestroyActor (Variables|Default|GetCurrentPickup)))))))

(event Custom|IdleCaddie
  (Components|Timeline|SetPlayRate (Variables|Default|GetTL_IdleCaddie) (/ 1.0 2.0))
  (bind _alpha (Timeline|TL_IdleCaddie PlayFromStart)
    (:Update
      (Transformation|SetWorldScale3D (Variables|Default|GetCube) (Math|Vector|Lerp(Vector) "1.000000,1.000000,1.000000" "1.050000,1.050000,1.050000" _alpha)))
    (:Finished
      (CallFunction|IdleCaddie))))

(event Custom|StartSlow
  (Variables|Default|SetIsSlowing true)
  (Variables|Defaults|SetSpeed "10.000000,0.000000,0.000000"))

(event Custom|Start
  (bind _returnvalue (Utilities|Time|SetTimerbyEvent (delegate Custom|Regen) 0.2)))

(event Custom|Regen
  (Variables|Default|SetRessource (Math|Float|Clamp(Float) (+ (Variables|Default|GetRessource) 5.0) 0.0 (Variables|Default|GetMaxRessource)))
  (if (== (Math|Float|Clamp(Float) (+ (Variables|Default|GetRessource) 5.0) 0.0 (Variables|Default|GetMaxRessource)) (Variables|Default|GetMaxRessource))
    (CallFunction|StopRegen)))

(event Custom|StopRegen
  (Utilities|Time|ClearandInvalidateTimerbyHandle (stale Custom|InitiateRegen _returnvalue))
  (Utilities|Time|ClearandInvalidateTimerbyHandle (stale Custom|Start _returnvalue)))

(event Custom|GoForward
  (Transformation|AddActorLocalOffset (+ (Transformation|GetActorForwardVector self) (Variables|Defaults|GetSpeed)) false false))

(event Custom|StopSlow
  (Variables|Default|SetIsSlowing false)
  (Variables|Defaults|SetSpeed "25.000000,0.000000,0.000000"))

(event Custom|RessourceCalc
  (if (Variables|Default|GetIsSlowing)
    (CallFunction|UseRessource)))

(event Custom|UseRessource
  (Variables|Default|SetRessource 0.0)
  (Variables|Default|SetNormalized_ressource (Math|Float|NormalizetoRange (Math|Float|Clamp(Float) (- (Variables|Default|GetRessource) 5.0) 0.0 (Variables|Default|GetMaxRessource)) 0.0 1.5e+02))
  (Development|PrintString (Utilities|String|ToString(Float) (Variables|Default|GetRessource)))
  (Utilities|FlowControl|RetriggerableDelay 0.1)
  (CallFunction|RessourceCalc)
  (if (<= (Variables|Default|GetRessource) 0.0)
    (CallFunction|StopSlow)
    (CallFunction|RessourceCalc)
    (CallFunction|InitiateRegen)
    (else
      (CallFunction|RessourceCalc))))

(event Custom|InitiateRegen
  (bind _returnvalue (Utilities|Time|SetTimerbyEvent (delegate Custom|Start) 0.3 true)))

(event Input|EnhancedActionEvents|EnhancedInputActionIA_Move
  (params (ActionValue :type Vector%202D%20Structure) (ElapsedSeconds :type Float%20%28double-precision%29) (TriggeredSeconds :type Float%20%28double-precision%29) (InputAction :type Input%20Action%20Object%20Reference :default "/Game/Blueprints/Character/Inputs/InputActions/IA_Move.IA_Move"))
  (Pawn|Input|AddMovementInput (Math|Vector|GetRightVector (Math|Rotator|MakeRotator 0.0 0.0 (.yaw (Transformation|GetActorRotation)))) (.x ActionValue) false))

(event Input|EnhancedActionEvents|EnhancedInputActionIA_Jump
  (params (ActionValue :type Boolean) (ElapsedSeconds :type Float%20%28double-precision%29) (TriggeredSeconds :type Float%20%28double-precision%29) (InputAction :type Input%20Action%20Object%20Reference :default "/Game/Blueprints/Character/Inputs/InputActions/IA_Jump.IA_Jump"))
  (:Triggered
    (Character|Jump)
    (Variables|/Script/Engine.CharacterMovementComponent|SetGravityScale (Variables|Character|GetCharacterMovement) 1.6))
  (:Completed
    (Character|StopJumping)
    (Variables|/Script/Engine.CharacterMovementComponent|SetGravityScale (Variables|Character|GetCharacterMovement) 1.3)))

(event Input|EnhancedActionEvents|EnhancedInputActionIA_Slow
  (params (ActionValue :type Boolean) (ElapsedSeconds :type Float%20%28double-precision%29) (TriggeredSeconds :type Float%20%28double-precision%29) (InputAction :type Input%20Action%20Object%20Reference :default "/Game/Blueprints/Character/Inputs/InputActions/IA_Slow.IA_Slow"))
  (:Started
    (CallFunction|StartSlow)
    (CallFunction|RessourceCalc)
    (Niagara|SetNiagaraVariable(Float) (Variables|Default|GetNS_CubeSmoke) "Smoke_Ammount" (Variables|Default|GetNormalized_ressource)))
  (:Completed
    (CallFunction|StopSlow)))

(event EventBeginPlay
  (Input|AddMappingContext (PlayerController|LocalPlayerSubsystems|GetEnhancedInputLocalPlayerSubsystem (Game|GetPlayerController 0)) "/Game/Blueprints/Character/Inputs/IMC_Chara.IMC_Chara" 0 "(bIgnoreAllPressedKeysUntilRelease=True,bForceImmediately=False,bNotifyUserSettings=False)")
  (Variables|/Script/Engine.CharacterMovementComponent|SetGravityScale (Variables|Character|GetCharacterMovement) 1.3)
  (bind _returnvalue (Actor|GetActorOfClass "/Game/Blueprints/Camera/BP_MainCamera.BP_MainCamera_C"))
  (Variables|Default|SetMainCamera _returnvalue)
  (Variables|Default|SetMaxRessource 1.5e+02)
  (Variables|Default|SetRessource 1.5e+02)
  (CallFunction|IdleCaddie)
  (Components|Activation|Deactivate (Variables|Default|GetNiagara))
  (Niagara|SetNiagaraVariable(Float) (Variables|Default|GetNS_CubeSmoke) "Smoke_Ammount" 1.0))

(event Collision|EventActorBeginOverlap
  (params (OtherActor :type Actor%20Object%20Reference)))

(event EventTick
  (params (DeltaSeconds :type Float%20%28single-precision%29))
  (CallFunction|GoForward))

(fn ConstructionScript)