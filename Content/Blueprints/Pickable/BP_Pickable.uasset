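; BP_Pickable is a moving pickable item that picks a random fruit, household or fresh product within its PickableType, setting its mesh and movement.
; Runners get repeated impulses toward a shuffled BP_TargetPointZone whenever they slow down.
; Jumpers turn via timeline, leap alternately away from and toward BP_Chara with Niagara effects, then repeat after stopping and a random delay.
; Others drift in looping timeline offsets; some jumpers spawn a BP_Flaque at start.
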(event Custom|StartJumping
  (bind _returnvalue (Transformation|GetActorLocation))
  (bind _player (Variables|References|GetPlayer))
  (bind _returnvalue_2 (Transformation|GetActorLocation _player))
  (bind _returnvalue_3 (- _returnvalue_2 _returnvalue))
  (bind _returnvalue_4 (Math|Vector|VectorLength _returnvalue_3))
  (bind _returnvalue_5 (Math|Float|MapRangeClamped _returnvalue_4 0.0 1e+04 1e+01 5e+01))
  ;[0.15 0.15 0.15 0.5] Movement Jump
  (bind _output_get (Variables|Jump|SetDirectionToJumpTo _returnvalue_3))
  (Utilities|FlowControl|FlipFlop
    (:A
      (Variables|Jump|SetImpulseJump (Math|Vector|MakeVector (.x (* (Math|Vector|MakeVector (.x (* _output_get (Math|Vector|MakeVector _returnvalue_5 _returnvalue_5 0.0))) (.y (* _output_get (Math|Vector|MakeVector _returnvalue_5 _returnvalue_5 0.0))) 0.0) -0.3)) (.y (* (Math|Vector|MakeVector (.x (* _output_get (Math|Vector|MakeVector _returnvalue_5 _returnvalue_5 0.0))) (.y (* _output_get (Math|Vector|MakeVector _returnvalue_5 _returnvalue_5 0.0))) 0.0) -0.3)) (Variables|Jump|GetThrowForceZMovementJump))))
    (:B
      (Variables|Jump|SetImpulseJump (Math|Vector|MakeVector (.x (* (Math|Vector|MakeVector (.x (* _output_get (Math|Vector|MakeVector _returnvalue_5 _returnvalue_5 0.0))) (.y (* _output_get (Math|Vector|MakeVector _returnvalue_5 _returnvalue_5 0.0))) 0.0) 0.3)) (.y (* (Math|Vector|MakeVector (.x (* _output_get (Math|Vector|MakeVector _returnvalue_5 _returnvalue_5 0.0))) (.y (* _output_get (Math|Vector|MakeVector _returnvalue_5 _returnvalue_5 0.0))) 0.0) 0.3)) (Variables|Jump|GetThrowForceZMovementJump)))))
  (Components|Timeline|SetPlayRate (Variables|Default|GetTL_Jump) (/ 1.0 0.2))
  (Variables|Jump|SetStartRotationJump (Transformation|GetWorldRotation (Variables|Default|GetSM)))
  (Variables|Jump|SetEndRotationJump (Math|Rotator|FindLookatRotation (- (Transformation|GetActorLocation (Variables|References|GetPlayer)) (Math|Vector|MakeVector 0.0 0.0 (Math|Float|MapRangeClamped (Math|Vector|Distance(Vector) (Transformation|GetActorLocation (Variables|References|GetPlayer)) (Transformation|GetActorLocation)) 0.0 3e+03 1.5e+03 0.0))) (Transformation|GetWorldLocation (Variables|Default|GetSM))))
  (bind _alpha (Timeline|TL_Jump PlayFromStart)
    (:Update
      (Transformation|SetWorldRotation (Variables|Default|GetSM) (Math|Rotator|Lerp(Rotator) (Variables|Jump|GetStartRotationJump) (Variables|Jump|GetEndRotationJump) _alpha true) false false))
    (:Finished
      (Components|Activation|Activate (Variables|Default|GetNiagara) true)
      (Physics|AddImpulse (Variables|Character|GetCharacterMovement) (Variables|Jump|GetImpulseJump) false)
      (CallFunction|TimerReJump)
      (Utilities|FlowControl|Delay 0.6)
      (Components|Activation|Deactivate (Variables|Default|GetNiagara)))))

(event Custom|TimerReJump
  ;[0.15 0.15 0.15 0.5] Movement Jump
  (bind _returnvalue (Utilities|Time|SetTimerbyEvent (delegate Custom|CodeTimerReJump) 0.1 true)))

(event Custom|CodeTimerReJump
  ;[0.15 0.15 0.15 0.5] Movement Jump
  (if (Utilities|Operators|EqualEqual :A (Variables|/Script/Engine.MovementComponent|GetVelocity (Variables|Character|GetCharacterMovement)))
    (Utilities|Time|ClearandInvalidateTimerbyHandle (stale Custom|TimerReJump _returnvalue))
    (Utilities|FlowControl|Delay (Math|Random|RandomFloatinRange (Variables|Jump|GetMinDelayBetweenJump) (Variables|Jump|GetMaxDelayBetweenJump)))
    (CallFunction|StartJumping)))

(event Custom|RunningMovement
  ;[0.15 0.15 0.15 0.5] Movement Run
  (bind _output_get (Variables|MovementRun|SetTempAllTargetPoints (Variables|References|GetAllTargetPoints)))
  (Utilities|Array|Shuffle _output_get)
  (if (Utilities|Array|IsValidIndex (Variables|MovementRun|GetTempAllTargetPoints))
    (Variables|MovementRun|SetCurrentTargetPoint (Utilities|Array|Get(acopy) (Variables|MovementRun|GetTempAllTargetPoints)))
    (CallFunction|StartMoving)
    (Utilities|Array|RemoveIndex (Variables|MovementRun|GetTempAllTargetPoints))
    (else
      (CallFunction|RunningMovement))))

(event Custom|StartMoving
  (bind _self self)
  (bind _currenttargetpoint (Variables|MovementRun|GetCurrentTargetPoint))
  (bind _returnvalue (Transformation|GetActorLocation _currenttargetpoint))
  (bind _returnvalue_2 (Transformation|GetActorLocation _self))
  (bind _returnvalue_3 (- _returnvalue _returnvalue_2))
  (bind _returnvalue_4 (Math|Vector|VectorLength _returnvalue_3))
  (bind _returnvalue_5 (Math|Float|MapRangeClamped _returnvalue_4 1e+03 2e+02 2e+01 8e+01))
  ;[0.15 0.15 0.15 0.5] Movement Run
  (Variables|Default|SetStartRotationMovementRun (Transformation|GetActorRotation self))
  (Variables|Default|SetEndRotationMovementRun (Math|Rotator|FindLookatRotation (Transformation|GetActorLocation self) (Transformation|GetActorLocation (Variables|MovementRun|GetCurrentTargetPoint))))
  (Physics|AddImpulse (Variables|Character|GetCharacterMovement) (* _returnvalue_3 (Math|Vector|MakeVector _returnvalue_5 _returnvalue_5 0.0)) false)
  (CallFunction|TimerRuningMovement))

(event Custom|TimerRuningMovement
  ;[0.15 0.15 0.15 0.5] Movement Run
  (bind _returnvalue (Utilities|Time|SetTimerbyEvent (delegate Custom|CodeTimerRuningMovement) 0.01 true)))

(event Custom|CodeTimerRuningMovement
  ;[0.15 0.15 0.15 0.5] Movement Run
  (if (< (Math|Vector|VectorLength (Variables|/Script/Engine.MovementComponent|GetVelocity (Variables|Character|GetCharacterMovement))) 1e+02)
    (Utilities|Time|ClearandInvalidateTimerbyHandle (stale Custom|TimerRuningMovement _returnvalue))
    (CallFunction|StartMoving)))

(event Custom|MovementFromTargetPoint
  ;[0.15 0.15 0.15 0.5] Movement Run
  (if (Utilities|Array|IsValidIndex (Variables|MovementRun|GetTempAllTargetPoints))
    (Variables|MovementRun|SetCurrentTargetPoint (Utilities|Array|Get(acopy) (Variables|MovementRun|GetTempAllTargetPoints)))
    (CallFunction|StartMoving)
    (Utilities|Array|RemoveIndex (Variables|MovementRun|GetTempAllTargetPoints))
    (else
      (CallFunction|RunningMovement))))

(event Custom|MoveLoc
  ;[0.15 0.15 0.15 0.5] ZIGZAG
  (bind _output_get (Variables|Default|SetBaseLoc (Transformation|GetActorLocation)))
  (Variables|Default|SetNewLoc (+ _output_get (Math|Vector|MakeVector (Math|Random|RandomFloatinRange 5e+01 7e+01) (Math|Random|RandomFloatinRange 2.0 5.0) 0.0)))
  (Components|Timeline|SetPlayRate (Variables|Default|GetTL_MoveViaRot) (/ 1.0 (Variables|Default|GetMoveViaRotPlayrate)))
  (bind _alpha (Timeline|TL_MoveViaRot PlayFromStart)
    (:Update
      (Transformation|SetActorLocation (Math|Vector|MakeVector (.x (Math|Vector|Lerp(Vector) (- (Variables|Default|GetBaseLoc) 1e+01) (+ (Variables|Default|GetNewLoc) 1e+01) _alpha)) (.y (Math|Vector|Lerp(Vector) (- (Variables|Default|GetBaseLoc) 1e+01) (+ (Variables|Default|GetNewLoc) 1e+01) _alpha)) 0.0) false false)
      (Transformation|AddActorLocalOffset (+ (Transformation|GetActorRightVector) "0.000000,7.000000,0.000000") false false))
    (:Finished
      (CallFunction|MoveLoc))))

(event EventBeginPlay
  (bind _returnvalue (Actor|GetActorOfClass "/Game/Blueprints/Character/BP_Chara.BP_Chara_C"))
  (Variables|References|SetPlayer _returnvalue)
  (Components|Activation|Deactivate (Variables|Default|GetNiagara))
  (switch Utilities|FlowControl|Switch|SwitchonE_PickableType (Variables|SelfData|GetPickableType)
    (:NewEnumerator0
      (switch Utilities|FlowControl|Switch|SwitchonE_FruitsType (.OutItem (Utilities|Array|Random (Variables|SelfData|GetFruitsType)))
        (:NewEnumerator0
          (Variables|SelfData|SetFruitsTypeChosen "NewEnumerator0")
          (Variables|MovementRun|SetForceMovementRun 25.0)
          (Variables|MovementRun|SetbUseTargetPoints true)
          (Variables|/Script/Engine.CharacterMovementComponent|SetGravityScale (Variables|Character|GetCharacterMovement) 0.5)
          (CallFunction|RunningMovement)
          (Components|SkeletalMesh|SetSkeletalMeshAsset (Variables|Character|GetMesh) "/Game/Art/Characters/Mesh/SKM_tomato.SKM_tomato")
          (Components|Animation|PlayAnimation (Variables|Character|GetMesh) "/Game/Art/Characters/Mesh/SKM_tomato_Anim.SKM_tomato_Anim" true))
        (:NewEnumerator1
          (Variables|SelfData|SetFruitsTypeChosen "NewEnumerator1")
          (Variables|Jump|SetThrowForceXYMovementJump (Math|Float|MapRangeClamped (Math|Vector|VectorLength (- (Transformation|GetActorLocation (Variables|References|GetPlayer)) (Transformation|GetActorLocation))) 1e+04 0.0 5e+02 2e+02))
          (Variables|Jump|SetThrowForceZMovementJump (Math|Random|RandomFloatinRange 1.9e+03 2.1e+03))
          (Variables|/Script/Engine.CharacterMovementComponent|SetGravityScale (Variables|Character|GetCharacterMovement) 1.0)
          (Variables|/Script/Engine.CharacterMovementComponent|SetMass (Variables|Character|GetCharacterMovement) 5.0)
          (CallFunction|StartJumping)
          (Components|SkeletalMesh|SetSkeletalMeshAsset (Variables|Character|GetMesh) "/Game/Art/Characters/Mesh/SKM_lemon.SKM_lemon"))
        (:NewEnumerator2
          (Variables|SelfData|SetFruitsTypeChosen "NewEnumerator2")
          (CallFunction|MoveLoc)
          (Components|SkeletalMesh|SetSkeletalMeshAsset (Variables|Character|GetMesh) "/Game/Art/Characters/Mesh/SKM_cauliflower.SKM_cauliflower"))
        (:NewEnumerator3
          (Utilities|FlowControl|Sequence
            (:then_0
              (Variables|SelfData|SetFruitsTypeChosen "NewEnumerator3")
              (Variables|Jump|SetThrowForceXYMovementJump (Math|Random|RandomFloatinRange 75.0 95.0))
              (Variables|Jump|SetThrowForceZMovementJump (Math|Random|RandomFloatinRange 1.9e+03 2.1e+03))
              (Variables|/Script/Engine.CharacterMovementComponent|SetGravityScale (Variables|Character|GetCharacterMovement) 1.0)
              (Variables|/Script/Engine.CharacterMovementComponent|SetMass (Variables|Character|GetCharacterMovement) 1e+01)
              (CallFunction|StartJumping)
              (Components|SkeletalMesh|SetSkeletalMeshAsset (Variables|Character|GetMesh) "/Game/Art/Characters/Mesh/SKM_banana.SKM_banana"))
            (:then_1
              (Utilities|FlowControl|DoOnce false
                (:Completed
                  (Game|SpawnActorfromClass "/Game/Blueprints/Enviro/BP_Flaque.BP_Flaque_C" (Transformation|GetActorTransform) "AdjustIfPossibleButAlwaysSpawn" "MultiplyWithRoot" 0 0))))))))
    (:NewEnumerator1
      (switch Utilities|FlowControl|Switch|SwitchonE_MenagerType (.OutItem (Utilities|Array|Random (Variables|SelfData|GetMenagerType)))
        (:NewEnumerator0
          (Variables|SelfData|SetMenagerTypeChosen "NewEnumerator0")
          (Variables|MovementRun|SetForceMovementRun 25.0)
          (Variables|MovementRun|SetbUseTargetPoints true)
          (Variables|/Script/Engine.CharacterMovementComponent|SetGravityScale (Variables|Character|GetCharacterMovement) 0.5)
          (CallFunction|RunningMovement)
          (Components|SkeletalMesh|SetSkeletalMeshAsset (Variables|Character|GetMesh) "/Game/Art/Characters/Mesh/SKM_soap.SKM_soap")
          (Components|Animation|PlayAnimation (Variables|Character|GetMesh) "/Game/Art/Characters/Mesh/SKM_tomato_Anim.SKM_tomato_Anim" true))
        (:NewEnumerator1
          (Variables|SelfData|SetMenagerTypeChosen "NewEnumerator1")
          (Variables|Jump|SetThrowForceXYMovementJump (Math|Float|MapRangeClamped (Math|Vector|VectorLength (- (Transformation|GetActorLocation (Variables|References|GetPlayer)) (Transformation|GetActorLocation))) 1e+04 0.0 5e+02 1e+02))
          (Variables|Jump|SetThrowForceZMovementJump (Math|Random|RandomFloatinRange 1.9e+03 2.1e+03))
          (Variables|/Script/Engine.CharacterMovementComponent|SetGravityScale (Variables|Character|GetCharacterMovement) 1.0)
          (Variables|/Script/Engine.CharacterMovementComponent|SetMass (Variables|Character|GetCharacterMovement) 1e+01)
          (Components|SkeletalMesh|SetSkeletalMeshAsset (Variables|Character|GetMesh) "/Game/Art/Characters/Mesh/SKM_pod.SKM_pod")
          (CallFunction|StartJumping))
        (:NewEnumerator2
          (Variables|SelfData|SetMenagerTypeChosen "NewEnumerator2")
          (CallFunction|MoveLoc)
          (Components|SkeletalMesh|SetSkeletalMeshAsset (Variables|Character|GetMesh) "/Game/Art/Characters/Mesh/SKM_bleach.SKM_bleach"))
        (:NewEnumerator3
          (Utilities|FlowControl|Sequence
            (:then_0
              (Variables|SelfData|SetMenagerTypeChosen "NewEnumerator3")
              (Variables|Jump|SetThrowForceXYMovementJump (Math|Random|RandomFloatinRange 1e+02 1.1e+02))
              (Variables|Jump|SetThrowForceZMovementJump (Math|Random|RandomFloatinRange 2e+03 2.2e+03))
              (Variables|/Script/Engine.CharacterMovementComponent|SetGravityScale (Variables|Character|GetCharacterMovement) 1.2)
              (Variables|/Script/Engine.CharacterMovementComponent|SetMass (Variables|Character|GetCharacterMovement) 3.0)
              (CallFunction|StartJumping)
              (Components|SkeletalMesh|SetSkeletalMeshAsset (Variables|Character|GetMesh) "/Game/Art/Characters/Mesh/SKM_bleach.SKM_bleach"))
            (:then_1
              (Game|SpawnActorfromClass "/Game/Blueprints/Enviro/BP_Flaque.BP_Flaque_C" (Transformation|GetActorTransform) "AdjustIfPossibleButAlwaysSpawn" "MultiplyWithRoot" 0 0))))))
    (:NewEnumerator2
      (switch Utilities|FlowControl|Switch|SwitchonE_FraisType (.OutItem (Utilities|Array|Random (Variables|SelfData|GetFraisType)))
        (:NewEnumerator0
          (Variables|SelfData|SetFraisTypeChosen "NewEnumerator0")
          (Variables|MovementRun|SetForceMovementRun 75.0)
          (Variables|MovementRun|SetbUseTargetPoints true)
          (Variables|/Script/Engine.CharacterMovementComponent|SetGravityScale (Variables|Character|GetCharacterMovement) 0.2)
          (CallFunction|RunningMovement)
          (Components|SkeletalMesh|SetSkeletalMeshAsset (Variables|Character|GetMesh) "/Game/Art/Characters/Mesh/SKM_icecream.SKM_icecream")
          (Components|Animation|PlayAnimation (Variables|Character|GetMesh) "/Game/Art/Characters/Mesh/SKM_tomato_Anim.SKM_tomato_Anim" true))
        (:NewEnumerator1
          (Variables|SelfData|SetFraisTypeChosen "NewEnumerator1")
          (Variables|Jump|SetThrowForceXYMovementJump 1e+02)
          (Variables|Jump|SetThrowForceZMovementJump 2e+03)
          (Variables|/Script/Engine.CharacterMovementComponent|SetGravityScale (Variables|Character|GetCharacterMovement) 1.0)
          (Variables|/Script/Engine.CharacterMovementComponent|SetMass (Variables|Character|GetCharacterMovement) 2.0)
          (CallFunction|StartJumping)
          (Components|SkeletalMesh|SetSkeletalMeshAsset (Variables|Character|GetMesh) "/Game/Art/Characters/Mesh/SKM_egg.SKM_egg"))
        (:NewEnumerator2
          (Variables|SelfData|SetFraisTypeChosen "NewEnumerator2")
          (CallFunction|MoveLoc)
          (Components|StaticMesh|SetStaticMesh (Variables|Default|GetSM) "/Game/Art/Characters/Mesh/milk.milk"))
        (:NewEnumerator3
          (Variables|SelfData|SetFraisTypeChosen "NewEnumerator3")
          (Utilities|FlowControl|Sequence
            (:then_0
              (Variables|Jump|SetThrowForceXYMovementJump (Math|Random|RandomFloatinRange 75.0 95.0))
              (Variables|Jump|SetThrowForceZMovementJump (Math|Random|RandomFloatinRange 1.8e+03 2e+03))
              (Variables|/Script/Engine.CharacterMovementComponent|SetGravityScale (Variables|Character|GetCharacterMovement) 0.8)
              (Variables|/Script/Engine.CharacterMovementComponent|SetMass (Variables|Character|GetCharacterMovement) 1.5)
              (CallFunction|StartJumping)
              (Components|SkeletalMesh|SetSkeletalMeshAsset (Variables|Character|GetMesh) 0))
            (:then_1
              (Utilities|FlowControl|DoOnce false
                (:Completed
                  (Game|SpawnActorfromClass "/Game/Blueprints/Enviro/BP_Flaque.BP_Flaque_C" (Transformation|GetActorTransform) "AdjustIfPossibleButAlwaysSpawn" "MultiplyWithRoot" 0 0))))))))))

(fn ConstructionScript
  (bind _outactors (Actor|GetAllActorsOfClass "/Game/Blueprints/Pickable/BP_TargetPointZone.BP_TargetPointZone_C"))
  (bind _output_get (Variables|References|SetAllTargetPoints _outactors))
  (Variables|MovementRun|SetTempAllTargetPoints _output_get))