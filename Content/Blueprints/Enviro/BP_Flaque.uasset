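; BP_Flaque is an environment puddle that alters a character's Speed while standing in it and expires after ten seconds.
; On Box overlap with a BP_Chara, it overwrites the Speed vector's X with half the vector's length, then with double the length on exit.
; BeginPlay calls DestroySelf, which sets the lifespan and prints a leftover debug string.
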(event OnComponentBeginOverlap(Box)
  (params (OverlappedComponent :type Primitive%20Component%20Object%20Reference) (OtherActor :type Actor%20Object%20Reference) (OtherComp :type Primitive%20Component%20Object%20Reference) (OtherBodyIndex :type Integer) (bFromSweep :type Boolean) (SweepResult :type Hit%20Result%20Structure%20%28by%20ref%29))
  (bind (_asbp_chara _bsuccess) (Utilities|Casting|CastToBP_Chara OtherActor))
  (bind _speed (Variables|/Game/Blueprints/Character/BP_Chara.BP_Chara_C|GetSpeed _asbp_chara))
  (if _bsuccess
    (Class|KismetMathLibrary|VectorSet _speed (/ (Math|Vector|VectorLength _speed) 2.0) 0.0 0.0)))

(event OnComponentEndOverlap(Box)
  (params (OverlappedComponent :type Primitive%20Component%20Object%20Reference) (OtherActor :type Actor%20Object%20Reference) (OtherComp :type Primitive%20Component%20Object%20Reference) (OtherBodyIndex :type Integer))
  (bind (_asbp_chara _bsuccess) (Utilities|Casting|CastToBP_Chara OtherActor))
  (bind _speed (Variables|/Game/Blueprints/Character/BP_Chara.BP_Chara_C|GetSpeed _asbp_chara))
  (if _bsuccess
    (Class|KismetMathLibrary|VectorSet _speed (* (Math|Vector|VectorLength _speed) 2.0) 0.0 0.0)))

(event Custom|DestroySelf
  (Actor|SetLifeSpan 1e+01)
  (Development|PrintString "Hello"))

(event EventBeginPlay
  (CallFunction|DestroySelf))

(event Collision|EventActorBeginOverlap
  (params (OtherActor :type Actor%20Object%20Reference)))

(event EventTick
  (params (DeltaSeconds :type Float%20%28single-precision%29)))

(fn ConstructionScript)