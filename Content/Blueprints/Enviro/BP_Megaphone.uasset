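; Environment megaphone actor that plays sounds at its location on spawn and when the player character touches it.
; On BeginPlay it plays a quiet cartoon music track with no attenuation override.
; When an actor of exactly class BP_Chara begins overlapping, it plays a random clip from its Sound array with attenuation settings.
; Both sounds get a slightly randomized pitch on each play.
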(event EventBeginPlay
  (Audio|PlaySoundatLocation "/Game/Art/Sounds/cartoon-music-soundtrack-cartoon-game-upgrade-494470.cartoon-music-soundtrack-cartoon-game-upgrade-494470" (Transformation|GetActorLocation) "0, 0, 0" 0.1 (Math|Random|RandomFloatinRange 0.8 1.2) 0.0 0 0 0 0))

(event Collision|EventActorBeginOverlap
  (params (OtherActor :type Actor%20Object%20Reference))
  (if (== (Utilities|GetClass OtherActor) "/Game/Blueprints/Character/BP_Chara.BP_Chara_C")
    (Audio|PlaySoundatLocation (.OutItem (Utilities|Array|Random (Variables|Default|GetSound))) (Transformation|GetActorLocation) "0, 0, 0" 0.4 (Math|Random|RandomFloatinRange 0.8 1.2) 0.0 "/Game/Blueprints/Enviro/Buhbuhbuh.Buhbuhbuh" 0 0 0)))

(fn ConstructionScript)