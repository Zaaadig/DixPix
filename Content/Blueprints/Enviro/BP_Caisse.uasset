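; BP_Caisse is an environment actor that acts as a win trigger for the player character.
; When an actor overlaps its Box while IsActive is true, it casts to BP_Chara and checks HasWin.
; If that flag is set, a DoOnce creates the WB_Win widget and adds it to the viewport.
; It also caches a BP_GameManager reference on BeginPlay, which this graph does not use afterwards.
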(event OnComponentBeginOverlap(Box)
  (params (OverlappedComponent :type Primitive%20Component%20Object%20Reference) (OtherActor :type Actor%20Object%20Reference) (OtherComp :type Primitive%20Component%20Object%20Reference) (OtherBodyIndex :type Integer) (bFromSweep :type Boolean) (SweepResult :type Hit%20Result%20Structure%20%28by%20ref%29))
  (if (Variables|Default|GetbIsActive)
    (bind _asbp_chara (Utilities|Casting|CastToBP_Chara OtherActor))
    (if (Variables|/Game/Blueprints/Character/BP_Chara.BP_Chara_C|GetbHasWin _asbp_chara)
      (Utilities|FlowControl|DoOnce false
        (:Completed
          (bind _returnvalue (UserInterface|CreateWidget "/Game/UI/WB_Win.WB_Win_C"))
          (UserInterface|Viewport|AddtoViewport _returnvalue 0))))))

(event EventBeginPlay
  (bind _returnvalue (Actor|GetActorOfClass "/Game/Blueprints/Manager/BP_GameManager.BP_GameManager_C"))
  (Variables|References|SetGameManager _returnvalue))

(fn ConstructionScript)