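; BP_accelerator is an environment trigger zone that boosts pickables and the player character while they are inside its box.
; On overlap, a BP_Pickable gets higher jump throw forces and run force, while a BP_Chara gets a higher Speed vector.
; Leaving the box writes fixed lower values back rather than restoring saved ones.
; The BP_Chara reference cached on BeginPlay is not used by the overlap logic.
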(event OnComponentBeginOverlap(Box)
  (params (OverlappedComponent :type Primitive%20Component%20Object%20Reference) (OtherActor :type Actor%20Object%20Reference) (OtherComp :type Primitive%20Component%20Object%20Reference) (OtherBodyIndex :type Integer) (bFromSweep :type Boolean) (SweepResult :type Hit%20Result%20Structure%20%28by%20ref%29))
  (bind _asbp_pickable (Utilities|Casting|CastToBP_Pickable OtherActor)
    (:then
      (Variables|Default|SetBp_Pickable _asbp_pickable)
      (Variables|/Game/Blueprints/Pickable/BP_Pickable.BP_Pickable_C|SetThrowForceXYMovementJump (Variables|Default|GetBp_Pickable) 7.5e+03)
      (Variables|/Game/Blueprints/Pickable/BP_Pickable.BP_Pickable_C|SetThrowForceZMovementJump (Variables|Default|GetBp_Pickable) 7.5e+03)
      (Variables|/Game/Blueprints/Pickable/BP_Pickable.BP_Pickable_C|SetForceMovementRun (Variables|Default|GetBp_Pickable) 1e+02))
    (:CastFailed
      (bind _asbp_chara (Utilities|Casting|CastToBP_Chara OtherActor))
      (Variables|/Game/Blueprints/Character/BP_Chara.BP_Chara_C|SetSpeed _asbp_chara "50.000000,0.000000,0.000000"))))

(event OnComponentEndOverlap(Box)
  (params (OverlappedComponent :type Primitive%20Component%20Object%20Reference) (OtherActor :type Actor%20Object%20Reference) (OtherComp :type Primitive%20Component%20Object%20Reference) (OtherBodyIndex :type Integer))
  (bind _asbp_pickable (Utilities|Casting|CastToBP_Pickable OtherActor)
    (:then
      (Variables|Default|SetBp_Pickable _asbp_pickable)
      (Variables|/Game/Blueprints/Pickable/BP_Pickable.BP_Pickable_C|SetThrowForceXYMovementJump (Variables|Default|GetBp_Pickable) 5e+03)
      (Variables|/Game/Blueprints/Pickable/BP_Pickable.BP_Pickable_C|SetThrowForceZMovementJump (Variables|Default|GetBp_Pickable) 5e+03)
      (Variables|/Game/Blueprints/Pickable/BP_Pickable.BP_Pickable_C|SetForceMovementRun (Variables|Default|GetBp_Pickable) 75.0))
    (:CastFailed
      (bind _asbp_chara (Utilities|Casting|CastToBP_Chara OtherActor))
      (Variables|/Game/Blueprints/Character/BP_Chara.BP_Chara_C|SetSpeed _asbp_chara "25.000000,0.000000,0.000000"))))

(event EventBeginPlay
  (bind _returnvalue (Actor|GetActorOfClass "/Game/Blueprints/Character/BP_Chara.BP_Chara_C"))
  (Variables|Default|SetBP_chara _returnvalue))

(event Collision|EventActorBeginOverlap
  (params (OtherActor :type Actor%20Object%20Reference)))

(event EventTick
  (params (DeltaSeconds :type Float%20%28single-precision%29)))

(fn ConstructionScript)