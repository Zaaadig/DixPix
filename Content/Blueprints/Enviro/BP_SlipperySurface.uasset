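; BP_SlipperySurface is an environment actor that makes characters slide while inside its box trigger.
; On begin overlap it removes ground friction and sharply lowers walking braking deceleration on any Character, and slightly reduces the Speed vector on BP_Chara.
; On end overlap it writes back fixed friction, braking and speed values rather than restoring whatever each character had before.
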(event OnComponentBeginOverlap(Box)
  (params (OverlappedComponent :type Primitive%20Component%20Object%20Reference) (OtherActor :type Actor%20Object%20Reference) (OtherComp :type Primitive%20Component%20Object%20Reference) (OtherBodyIndex :type Integer) (bFromSweep :type Boolean) (SweepResult :type Hit%20Result%20Structure%20%28by%20ref%29))
  (Utilities|FlowControl|Sequence
    (:then_0
      (bind _ascharacter (Utilities|Casting|CastToCharacter OtherActor))
      (Variables|/Script/Engine.CharacterMovementComponent|SetGroundFriction (Variables|/Script/Engine.Character|GetCharacterMovement _ascharacter) 0.0)
      (Variables|/Script/Engine.CharacterMovementComponent|SetBrakingDecelerationWalking (Variables|/Script/Engine.Character|GetCharacterMovement _ascharacter) 5e+01))
    (:then_1
      (bind _asbp_chara (Utilities|Casting|CastToBP_Chara OtherActor))
      (Variables|/Game/Blueprints/Character/BP_Chara.BP_Chara_C|SetSpeed _asbp_chara "20.000000,0.000000,0.000000"))))

(event OnComponentEndOverlap(Box)
  (params (OverlappedComponent :type Primitive%20Component%20Object%20Reference) (OtherActor :type Actor%20Object%20Reference) (OtherComp :type Primitive%20Component%20Object%20Reference) (OtherBodyIndex :type Integer))
  (Utilities|FlowControl|Sequence
    (:then_0
      (bind _ascharacter (Utilities|Casting|CastToCharacter OtherActor))
      (Variables|/Script/Engine.CharacterMovementComponent|SetGroundFriction (Variables|/Script/Engine.Character|GetCharacterMovement _ascharacter) 8.0)
      (Variables|/Script/Engine.CharacterMovementComponent|SetBrakingDecelerationWalking (Variables|/Script/Engine.Character|GetCharacterMovement _ascharacter) 2048.0))
    (:then_1
      (bind _asbp_chara (Utilities|Casting|CastToBP_Chara OtherActor))
      (Variables|/Game/Blueprints/Character/BP_Chara.BP_Chara_C|SetSpeed _asbp_chara "25.000000,0.000000,0.000000"))))

(event EventBeginPlay)

(event Collision|EventActorBeginOverlap
  (params (OtherActor :type Actor%20Object%20Reference)))

(event EventTick
  (params (DeltaSeconds :type Float%20%28single-precision%29)))

(fn ConstructionScript)