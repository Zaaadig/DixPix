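; Store aisle that builds two facing rows of shelves and starts their content when the player character enters its trigger box.
; The construction script previews the rows as mesh instances, spaced by mesh width and DistanceBetweenRow.
; On BeginPlay, each instance becomes a BP_Etagere in a per-type array (Fruits, Menager, Frais), then the instanced mesh is destroyed.
; A BP_Chara overlap calls Start on that row type's shelves; Frais spawns leave Type at default.
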(event OnComponentBeginOverlap(Box)
  (params (OverlappedComponent :type Primitive%20Component%20Object%20Reference) (OtherActor :type Actor%20Object%20Reference) (OtherComp :type Primitive%20Component%20Object%20Reference) (OtherBodyIndex :type Integer) (bFromSweep :type Boolean) (SweepResult :type Hit%20Result%20Structure%20%28by%20ref%29))
  (Utilities|Casting|CastToBP_Chara OtherActor)
  (CallFunction|StartSpawnElements))

(event Custom|StartSpawnElements
  (switch Utilities|FlowControl|Switch|SwitchonE_PickableType (Variables|Data|GetTypeOfRow)
    (:NewEnumerator0
      (for _array_element (Variables|Default|GetAllBP_Etagere_Fruits)
        (Default|Start _array_element)))
    (:NewEnumerator1
      (for _array_element_2 (Variables|Default|GetAllBP_Etagere_Menager)
        (Default|Start _array_element_2)))
    (:NewEnumerator2
      (for _array_element_3 (Variables|Default|GetAllBP_Etagere_Frais)
        (Default|Start _array_element_3)))))

(event EventBeginPlay
  (switch Utilities|FlowControl|Switch|SwitchonE_PickableType (Variables|Data|GetTypeOfRow)
    (:NewEnumerator0
      (for _array_element (Variables|Default|GetAllInstances)
        (bind _returnvalue (Game|SpawnActorfromClass "/Game/Blueprints/Environnement/BP_Etagere.BP_Etagere_C" (.OutInstanceTransform (Components|InstancedStaticMesh|GetInstanceTransform (Variables|Default|GetInstancedStaticMesh) _array_element true)) "AdjustIfPossibleButAlwaysSpawn" "MultiplyWithRoot" 0 "NewEnumerator0" 0))
        (Utilities|Array|Add (Variables|Default|GetAllBP_Etagere_Fruits) _returnvalue)
        (Utilities|FlowControl|Delay 0.2)
        (Components|DestroyComponent (Variables|Default|GetInstancedStaticMesh))))
    (:NewEnumerator1
      (for _array_element_2 (Variables|Default|GetAllInstances)
        (bind _returnvalue_2 (Game|SpawnActorfromClass "/Game/Blueprints/Environnement/BP_Etagere.BP_Etagere_C" (.OutInstanceTransform (Components|InstancedStaticMesh|GetInstanceTransform (Variables|Default|GetInstancedStaticMesh) _array_element_2 true)) "AdjustIfPossibleButAlwaysSpawn" "MultiplyWithRoot" 0 "NewEnumerator1" 0))
        (Utilities|Array|Add (Variables|Default|GetAllBP_Etagere_Menager) _returnvalue_2)
        (Utilities|FlowControl|Delay 0.2)
        (Components|DestroyComponent (Variables|Default|GetInstancedStaticMesh))))
    (:NewEnumerator2
      (for _array_element_3 (Variables|Default|GetAllInstances)
        (bind _returnvalue_3 (Game|SpawnActorfromClass "/Game/Blueprints/Environnement/BP_Etagere.BP_Etagere_C" (.OutInstanceTransform (Components|InstancedStaticMesh|GetInstanceTransform (Variables|Default|GetInstancedStaticMesh) _array_element_3 true)) "AdjustIfPossibleButAlwaysSpawn" "MultiplyWithRoot" 0 "NewEnumerator2" 0))
        (Utilities|Array|Add (Variables|Default|GetAllBP_Etagere_Frais) _returnvalue_3)
        (Utilities|FlowControl|Delay 0.2)
        (Components|DestroyComponent (Variables|Default|GetInstancedStaticMesh))))))

(fn ConstructionScript
  (bind _instancedstaticmesh (Variables|Default|GetInstancedStaticMesh))
  (bind _instancedstaticmesh_2 (Variables|Default|GetInstancedStaticMesh))
  (bind _staticmesh (Variables|/Script/Engine.StaticMeshComponent|GetStaticMesh _instancedstaticmesh))
  (bind _staticmesh_2 (Variables|/Script/Engine.StaticMeshComponent|GetStaticMesh _instancedstaticmesh_2))
  (bind _returnvalue (StaticMesh|GetBoundingBox _staticmesh))
  (bind _returnvalue_2 (StaticMesh|GetBoundingBox _staticmesh_2))
  (Components|StaticMesh|SetStaticMesh (Variables|Default|GetInstancedStaticMesh) (Variables|Data|GetStaticMesh))
  (Utilities|FlowControl|Sequence
    (:then_0
      (for _index (range 0 (Variables|Data|GetNmbr_Etageres))
        (bind _returnvalue_3 (Components|InstancedStaticMesh|AddInstance (Variables|Default|GetInstancedStaticMesh) (Math|Transform|MakeTransform (Math|Vector|MakeVector (* _index (.x (- (.max _returnvalue_2) (.min _returnvalue_2)))) 0.0 0.0) "0.000000,90.000000,0.000000" "1.000000,0.500000,1.000000") false))
        (Utilities|Array|Add (Variables|Default|GetAllInstances) _returnvalue_3)))
    (:then_1
      (for _index_2 (range 0 (Variables|Data|GetNmbr_Etageres))
        (bind _returnvalue_4 (Components|InstancedStaticMesh|AddInstance (Variables|Default|GetInstancedStaticMesh) (Math|Transform|MakeTransform (Math|Vector|MakeVector (* _index_2 (.x (- (.max _returnvalue) (.min _returnvalue)))) (Variables|Data|GetDistanceBetweenRow) 0.0) "0.000000,-90.000000,0.000000" "1.000000,0.500000,1.000000") false))
        (Utilities|Array|Add (Variables|Default|GetAllInstances) _returnvalue_4)))))