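; BP_Couloir is an environment Blueprint that builds a straight corridor from a single instanced static mesh.
; The Construction Script adds two parallel rows of ten instances in local space, offset along Y, rotated in opposite directions and scaled to half on Y.
; Spacing along X comes from the mesh's bounding-box X size.
; The event graph holds no gameplay logic.
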(event EventBeginPlay)

(event Collision|EventActorBeginOverlap
  (params (OtherActor :type Actor%20Object%20Reference)))

(event EventTick
  (params (DeltaSeconds :type Float%20%28single-precision%29)))

(fn ConstructionScript
  (bind _instancedstaticmesh (Variables|Default|GetInstancedStaticMesh))
  (bind _instancedstaticmesh_2 (Variables|Default|GetInstancedStaticMesh))
  (bind _staticmesh (Variables|/Script/Engine.StaticMeshComponent|GetStaticMesh _instancedstaticmesh))
  (bind _staticmesh_2 (Variables|/Script/Engine.StaticMeshComponent|GetStaticMesh _instancedstaticmesh_2))
  (bind _returnvalue (StaticMesh|GetBoundingBox _staticmesh))
  (bind _returnvalue_2 (StaticMesh|GetBoundingBox _staticmesh_2))
  (Utilities|FlowControl|Sequence
    (:then_0
      (for _index (range 0 9)
        (Components|InstancedStaticMesh|AddInstance (Variables|Default|GetInstancedStaticMesh) (Math|Transform|MakeTransform (Math|Vector|MakeVector (* _index (.x (- (.max _returnvalue_2) (.min _returnvalue_2)))) 0.0 0.0) "0.000000,90.000000,0.000000" "1.000000,0.500000,1.000000") false)))
    (:then_1
      (for _index_2 (range 0 9)
        (Components|InstancedStaticMesh|AddInstance (Variables|Default|GetInstancedStaticMesh) (Math|Transform|MakeTransform (Math|Vector|MakeVector (* _index_2 (.x (- (.max _returnvalue) (.min _returnvalue)))) 7.8e+02 0.0) "0.000000,-90.000000,0.000000" "1.000000,0.500000,1.000000") false)))))