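; BP_Etagere is a shelf actor that ejects a single BP_Pickable shortly after play begins.
; Its Menager or Frais type sets the pickable's gravity and movement tuning, though both spawn a Frais pickable and use the same fridge mesh.
; The pickable spawns tiny at the Arrow and gets an impulse from its forward vector while a timeline scales it up.
; After a short delay, it starts running (Menager) or jumping (Frais).
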(event Custom|StartDroppingItem
  (bind _arrow (Variables|Default|GetArrow))
  (bind _arrow_2 (Variables|Default|GetArrow))
  (bind _returnvalue (Transformation|GetWorldTransform _arrow_2))
  (bind _returnvalue_2 (Transformation|GetWorldTransform _arrow))
  (switch Utilities|FlowControl|Switch|SwitchonE_PickableType (Variables|Default|GetType)
    (:NewEnumerator1
      (bind _outactors (Actor|GetAllActorsOfClass "/Game/Blueprints/Pickable/BP_TargetPointZone.BP_TargetPointZone_C"))
      (Variables|Default|SetTargetPointRef _outactors)
      (bind _returnvalue_3 (Game|SpawnActorfromClass "/Game/Blueprints/Pickable/BP_Pickable.BP_Pickable_C" (Math|Transform|MakeTransform (.location _returnvalue) (.rotation _returnvalue) "0.010000,0.010000,0.010000") "AdjustIfPossibleButAlwaysSpawn" "MultiplyWithRoot" 0 "NewEnumerator2" 0))
      (bind _output_get (Variables|Default|SetCurrentSpawnPickable _returnvalue_3))
      (Variables|/Game/Blueprints/Pickable/BP_Pickable.BP_Pickable_C|SetForceMovementRun _output_get 15.0)
      (Variables|/Game/Blueprints/Pickable/BP_Pickable.BP_Pickable_C|SetFruitsTypeChosen _output_get "NewEnumerator2")
      (Variables|/Script/Engine.CharacterMovementComponent|SetGravityScale (Variables|/Script/Engine.Character|GetCharacterMovement _output_get) 0.2))
    (:NewEnumerator2
      (bind _returnvalue_4 (Game|SpawnActorfromClass "/Game/Blueprints/Pickable/BP_Pickable.BP_Pickable_C" (Math|Transform|MakeTransform (.location _returnvalue_2) (.rotation _returnvalue_2) "0.010000,0.010000,0.010000") "AdjustIfPossibleButAlwaysSpawn" "MultiplyWithRoot" 0 "NewEnumerator2" 0))
      (Variables|Default|SetCurrentSpawnPickable _returnvalue_4)
      (Variables|/Game/Blueprints/Pickable/BP_Pickable.BP_Pickable_C|SetThrowForceXYMovementJump (Variables|Default|GetCurrentSpawnPickable) 2e+01)
      (Variables|/Game/Blueprints/Pickable/BP_Pickable.BP_Pickable_C|SetThrowForceZMovementJump (Variables|Default|GetCurrentSpawnPickable) 1e+04)
      (Variables|/Script/Engine.CharacterMovementComponent|SetGravityScale (Variables|/Script/Engine.Character|GetCharacterMovement (Variables|Default|GetCurrentSpawnPickable)) 1.0)))
  (Physics|AddImpulse (Variables|/Script/Engine.Character|GetCharacterMovement (Variables|Default|GetCurrentSpawnPickable)) (* (Math|Vector|GetForwardVector (Variables|Default|GetArrow)) (Math|Vector|MakeVector 2e+02 2e+02 1e+03)) false)
  (Variables|Default|SetStartScaleSpawnPickable (Transformation|GetActorScale3D (Variables|Default|GetCurrentSpawnPickable)))
  (Components|Timeline|SetPlayRate (Variables|Default|GetTL_SpawnPickable) (/ 1.0 0.7))
  (bind _alpha (Timeline|TL_SpawnPickable PlayFromStart)
    (:Update
      (Transformation|SetActorScale3D (Variables|Default|GetCurrentSpawnPickable) (Math|Vector|Lerp(Vector) (Variables|Default|GetStartScaleSpawnPickable) "1.000000,1.000000,1.000000" _alpha)))
    (:Finished
      (Utilities|FlowControl|Delay 1.0)
      (switch Utilities|FlowControl|Switch|SwitchonE_PickableType (Variables|Default|GetType)
        (:NewEnumerator1
          (Default|RunningMovement (Variables|Default|GetCurrentSpawnPickable)))
        (:NewEnumerator2
          (Default|StartJumping (Variables|Default|GetCurrentSpawnPickable)))))))

(event EventBeginPlay
  (Utilities|FlowControl|Delay 1.0)
  (CallFunction|StartDroppingItem))

(event Collision|EventActorBeginOverlap
  (params (OtherActor :type Actor%20Object%20Reference)))

(event EventTick
  (params (DeltaSeconds :type Float%20%28single-precision%29)))

(fn ConstructionScript
  (switch Utilities|FlowControl|Switch|SwitchonE_PickableType (Variables|Default|GetType)
    (:NewEnumerator1
      _)
    (:NewEnumerator2
      _))
  (Components|StaticMesh|SetStaticMesh (Variables|Default|GetSM) "/Game/Art/Props/SM_Frigo_Full.SM_Frigo_Full"))