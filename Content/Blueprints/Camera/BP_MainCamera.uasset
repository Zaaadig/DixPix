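; BP_MainCamera is the main gameplay camera that takes over player 0's view when play begins.
; It finds the BP_Chara actor, moves its camera component to that character's Arrow1 world transform, then attaches itself to the character with world transforms kept.
; All setup happens once on BeginPlay, with no per-frame logic, so following relies on the attachment.
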(event EventBeginPlay
  (Game|Player|SetViewTargetwithBlend (Game|GetPlayerController 0) self 0.0 "VTBlend_Linear" 0.0 false)
  (bind _returnvalue (Actor|GetActorOfClass "/Game/Blueprints/Character/BP_Chara.BP_Chara_C"))
  (Transformation|SetWorldLocationAndRotation (Variables|CameraActor|GetCameraComponent self) (Transformation|GetWorldLocation (Variables|/Game/Blueprints/Character/BP_Chara.BP_Chara_C|GetArrow1 _returnvalue)) (Transformation|GetWorldRotation (Variables|/Game/Blueprints/Character/BP_Chara.BP_Chara_C|GetArrow1 _returnvalue)) false false)
  (Transformation|AttachActorToActor self _returnvalue "None" "KeepWorld" "KeepWorld" "KeepWorld" true))

(event Collision|EventActorBeginOverlap
  (params (OtherActor :type Actor%20Object%20Reference)))

(event EventTick
  (params (DeltaSeconds :type Float%20%28single-precision%29)))

(fn ConstructionScript)